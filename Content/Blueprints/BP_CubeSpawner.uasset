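; BP_CubeSpawner is an actor that periodically spawns BP_MyCube cubes around its own location.
; BeginPlay starts a looping five-second timer, and the Spawn event asks the Factory held by BP_GameMode to create each cube at a random horizontal offset, then prints its name.
; The timer is cleared when the spawner is destroyed.
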(event Custom|Spawn
  (bind _asbp_game_mode (Utilities|Casting|CastToBP_GameMode (Game|GetGameMode)))
  (bind _returnvalue (Class|CubeFactory|Create (Variables|/Game/Blueprints/BP_GameMode.BP_GameMode_C|GetFactory _asbp_game_mode) "/Game/Blueprints/BP_MyCube.BP_MyCube_C" (+ (Transformation|GetActorLocation) (Math|Vector|MakeVector (Math|Random|RandomFloatinRange -1.5e+02 1.5e+02) (Math|Random|RandomFloatinRange -1.5e+02 1.5e+02) 0.0)) "0, 0, 0"))
  (Development|PrintString (Utilities|GetDisplayName _returnvalue)))

(event EventBeginPlay
  (bind _returnvalue (Utilities|Time|SetTimerbyEvent (EventDispatchers|CreateEvent :!event Custom|Spawn) 5.0 true))
  (Variables|Default|SetTimer _returnvalue))

(event Collision|EventActorBeginOverlap
  (params (OtherActor :type Actor%20Object%20Reference)))

(event EventTick
  (params (DeltaSeconds :type Float%20%28single-precision%29)))

(event EventDestroyed
  (Utilities|Time|ClearandInvalidateTimerbyHandle (Variables|Default|GetTimer)))

(fn ConstructionScript)